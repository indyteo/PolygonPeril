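; Turret actor that automatically fires projectiles at the nearest enemy within its range.
; A sphere detector sized by Range and the actor overlap events maintain a list of actors implementing the Enemy interface.
; A looping cooldown timer spawns a projectile aimed at the nearest one, passing damage, speed, gravity and a homing target.
; The timer pauses when the last enemy leaves and resumes when another enters.
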(event `self.ReceiveBeginPlay`
  (`SphereComponent.SetSphereRadius` (`self.RangeDetector`) (`self.Range`) true)
  (bind _returnvalue (`KismetSystemLibrary.K2_SetTimerDelegate` (delegate `TurretMayShootEvent`) (`self.ShootCooldown`) true))
  (set `self.ShootTimer` _returnvalue)
  (for _array_element (`self.GetOverlappingActors` "/Script/Engine.Pawn")
    (if (`KismetSystemLibrary.DoesImplementInterface` _array_element "/Game/Blueprints/Enemy.Enemy_C")
      (`KismetArrayLibrary.Array_AddUnique` (`self.OverlappingEnemies`) _array_element))))

(event `TurretMayShootEvent`
  (bind _returnvalue (`SceneComponent.K2_GetComponentLocation` (`self.RangeDetector`)))
  (bind (_distance _returnvalue_2) (`GameplayStatics.FindNearestActor` _returnvalue (`self.OverlappingEnemies`)))
  (if (`KismetSystemLibrary.IsValid` _returnvalue_2)
    (`|SpawnActorFromClass` "/Game/Blueprints/Projectile.Projectile_C" (`KismetMathLibrary.MakeTransform` _returnvalue (`KismetMathLibrary.FindLookAtRotation` _returnvalue (`self.K2_GetActorLocation` _returnvalue_2))) "AlwaysSpawn" "OverrideRootScale" null (`self.Damage`) (`self.Speedness`) (`self.Gravity`) (`Actor.RootComponent` _returnvalue_2) null)))

(event `self.ReceiveActorBeginOverlap`
  (params (OtherActor :type "Actor Object Reference"))
  (if (`KismetSystemLibrary.DoesImplementInterface` OtherActor "/Game/Blueprints/Enemy.Enemy_C")
    (`KismetArrayLibrary.Array_AddUnique` (`self.OverlappingEnemies`) OtherActor)
    (if (`KismetSystemLibrary.K2_IsTimerPausedHandle` (`self.ShootTimer`))
      (`KismetSystemLibrary.K2_UnPauseTimerHandle` (`self.ShootTimer`)))))

(event `self.ReceiveActorEndOverlap`
  (params (OtherActor :type "Actor Object Reference"))
  (if (`KismetSystemLibrary.DoesImplementInterface` OtherActor "/Game/Blueprints/Enemy.Enemy_C")
    (`KismetArrayLibrary.Array_RemoveItem` (`self.OverlappingEnemies`) OtherActor)
    (if (and (not (`KismetSystemLibrary.K2_IsTimerPausedHandle` (`self.ShootTimer`))) (== 0 (`KismetArrayLibrary.Array_Length` (`self.OverlappingEnemies`))))
      (`KismetSystemLibrary.K2_PauseTimerHandle` (`self.ShootTimer`)))))

(fn `UserConstructionScript`)