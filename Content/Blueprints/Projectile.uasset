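; Projectile actor that damages enemies on hit, with configurable speed, gravity and optional homing.
; On BeginPlay it launches along the collision component's forward axis and applies speed and gravity to its projectile movement component.
; If a homing target component is valid, it homes with acceleration scaled from speed.
; Hitting an actor with the Enemy interface sends DamageMessage and destroys the projectile; other hits are ignored.
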(event `self.ReceiveBeginPlay`
  (bind _projectile (`self.Projectile`))
  (set `MovementComponent.Velocity` (`KismetMathLibrary.GreaterGreater_VectorRotator` (`KismetMathLibrary.MakeVector` (`self.Speedness`)) (`SceneComponent.K2_GetComponentRotation` (`self.CollisionComponent`))) _projectile)
  (set `ProjectileMovementComponent.InitialSpeed` (`self.Speedness`) _projectile)
  (set `ProjectileMovementComponent.MaxSpeed` (`self.Speedness`) _projectile)
  (set `ProjectileMovementComponent.ProjectileGravityScale` (`self.Gravity`) _projectile)
  (`/Engine/EditorBlueprintResources/StandardMacros.IsValid` (`self.Homing Target Component`)
    (:`Is Valid`
      (set `ProjectileMovementComponent.bIsHomingProjectile` true _projectile)
      (set `ProjectileMovementComponent.HomingAccelerationMagnitude` (* 100 (`self.Speedness`)) _projectile)
      (set `ProjectileMovementComponent.HomingTargetComponent` (`self.Homing Target Component`) _projectile))))

(event `self.ReceiveHit`
  (params (MyComp :type "PrimitiveComponent Object Reference") (Other :type "Actor Object Reference") (OtherComp :type "PrimitiveComponent Object Reference") (bSelfMoved :type Boolean) (HitLocation :type "Vector Structure") (HitNormal :type "Vector Structure") (NormalImpulse :type "Vector Structure") (Hit :type "HitResult Structure (by ref)"))
  (if (`KismetSystemLibrary.DoesImplementInterface` Other "/Game/Blueprints/Enemy.Enemy_C")
    (message `/Game/Blueprints/Enemy.Damage` Other (`self.Damage`))
    (`self.K2_DestroyActor`)))

(fn `UserConstructionScript`)