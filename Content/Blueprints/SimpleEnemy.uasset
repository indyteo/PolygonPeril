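; SimpleEnemy is an AI-driven enemy that moves on a target and drops coins when killed.
; On BeginPlay it sets full health, tints its sphere green through a dynamic material and passes the target's location to its EnemyController once.
; Damage reduces health and blends the color toward red by remaining health.
; At zero health it spawns a Coin carrying the drop value and destroys itself.
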(event `self.ReceiveBeginPlay`
  (set `self.Health` (`self.MaxHealth`))
  (bind _returnvalue (`PrimitiveComponent.CreateDynamicMaterialInstance` (`self.Sphere`) 0 "/Game/Blueprints/EnemyMaterial.EnemyMaterial" "Material"))
  (bind _output_get (set `self.Material` _returnvalue))
  (`MaterialInstanceDynamic.SetVectorParameterValue` _output_get "Color" (struct :`G` 1.0 :`A` 1.0))
  (bind _asenemy_controller (cast `/Game/Blueprints/EnemyController` (`AIBlueprintHelperLibrary.GetAIController` self)))
  (`/Game/Blueprints/EnemyController.SetTarget` _asenemy_controller (`self.K2_GetActorLocation` (`self.target`))))

(event `/Game/Blueprints/Enemy.Damage`
  (params (Amount :type "Float (single-precision)"))
  (bind _output_get (set `self.Health` (`KismetMathLibrary.FMax` (- (`self.Health`) Amount))))
  (if (<= _output_get 0.0)
    (`|SpawnActorFromClass` "/Game/Blueprints/Coin.Coin_C" (`self.GetTransform`) "AlwaysSpawn" "OverrideRootScale" null (`self.CoinsDroppedOnDeath`) null)
    (`self.K2_DestroyActor`)
    (else
      (`MaterialInstanceDynamic.SetVectorParameterValue` (`self.Material`) "Color" (`KismetMathLibrary.LinearColorLerp` (struct :`R` 1.0 :`A` 1.0) (struct :`G` 1.0 :`A` 1.0) (/ (`self.Health`) (`self.MaxHealth`)))))))

(fn `UserConstructionScript`)