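; TurretSlot is a placement point in the world where a turret can be built, managed or removed.
; On Interact it shows the interactor either the menu for its existing Turret or a new-turret menu for the empty slot.
; BuildTurret spawns the chosen class at the slot's transform, ignoring collisions, and stores it; DestroyTurret destroys the stored actor.
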(event `/Game/Blueprints/Interactable.Interact`
  (params (Interactor :type "/Game/FirstPersonBP/Blueprints/FirstPersonCharacter Object Reference"))
  (bind _turret (`self.Turret`))
  (`/Engine/EditorBlueprintResources/StandardMacros.IsValid` _turret
    (:`Is Valid`
      (`/Game/FirstPersonBP/Blueprints/FirstPersonCharacter.ShowTurretMenu` Interactor _turret))
    (:`Is Not Valid`
      (`/Game/FirstPersonBP/Blueprints/FirstPersonCharacter.ShowNewTurretMenu` Interactor self))))

(fn `BuildTurret`
  (params (Type :type "/Game/Blueprints/Turret Class Reference"))
  (bind _returnvalue (`|SpawnActorFromClass` Type (`self.GetTransform`) "AlwaysSpawn" "OverrideRootScale" null null))
  (set `self.Turret` _returnvalue))

(fn `DestroyTurret`
  (`self.K2_DestroyActor` (`self.Turret`)))

(fn `UserConstructionScript`)